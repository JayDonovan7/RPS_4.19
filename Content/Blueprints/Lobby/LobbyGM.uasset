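; Lobby game mode that manages joining players, character selection, match settings, kicking and map travel.
; PostLogin registers each controller, sets up its LobbyPC menu from GameInfoInstance and possesses a base character at a random PlayerStart.
; EveryoneUpdate sends player info and available characters to all LobbyPCs, blocking game start while anyone remains the base character.
; Settings changes propagate to every client, LaunchGame server-travels by map ID, and logout updates character availability.
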(event Custom|SwapCharacter
  (params (PlayerController :type Player%20Controller%20Object%20Reference) (CharacterClass :type Character%20Class%20Reference) (ChangedStatus :type Boolean))
  (bind _returnvalue (Pawn|GetControlledPawn PlayerController))
  (bind _spawnpoints (Variables|ServerSettings|GetSpawnPoints))
  ;[1 1 1] Swaps character from current to selected
  (if (not ChangedStatus)
    (Utilities|IsValid _returnvalue
      (:Is%20Valid
        (Actor|DestroyActor _returnvalue))
      (:Is%20Not%20Valid
        (bind _returnvalue_2 (Game|SpawnActorfromClass CharacterClass (Transformation|GetActorTransform (Utilities|Array|Get(acopy) _spawnpoints (Math|Random|RandomIntegerinRange 0 (- (Utilities|Array|Length _spawnpoints) 1)))) "Undefined" _returnvalue 0))
        (Pawn|Possess PlayerController _returnvalue_2)))))

(event Custom|EveryoneUpdate
  (bind _allplayercontrollers (Variables|ServerSettings|GetAllPlayerControllers))
  ;[1 1 1] Updates on connected player's lobby info
  (bind _output_get (Variables|ServerSettings|SetCurrent%20Players (Utilities|Array|Length (Variables|ServerSettings|GetAllPlayerControllers))))
  (if (> _output_get 0)
    (Utilities|Array|Clear (Variables|ServerSettings|GetConnectedPlayers))
    (for _array_element _allplayercontrollers
      (bind _aslobby_pc (Utilities|Casting|CastToLobbyPC _array_element))
      (Utilities|Array|Add (Variables|ServerSettings|GetConnectedPlayers) (Variables|/Game/Blueprints/Lobby/LobbyPC.LobbyPC_C|GetPlayerSettings _aslobby_pc))
      (Default|UpdateNumberOfPlayers _aslobby_pc (Variables|ServerSettings|GetCurrent%20Players) (Variables|ServerSettings|GetMax%20Players)))
    (for _array_element_2 _allplayercontrollers
      (bind _aslobby_pc_2 (Utilities|Casting|CastToLobbyPC _array_element_2))
      (Default|AddPlayerInfo _aslobby_pc_2 (Variables|ServerSettings|GetConnectedPlayers))
      (Default|UpdateAvailableCharacters _aslobby_pc_2 (Variables|ServerSettings|GetAvailable%20Characters))
      (CallFunction|AddtoKickList))
    (bind _array_element_3 (Utilities|Array|ForEachLoopwithBreak (Variables|ServerSettings|GetConnectedPlayers))
      (:LoopBody
        (if (== (.MyPlayerCharacter (Utilities|Struct|BreakPlayerInfo _array_element_3)) "/Game/Blueprints/Characters/0BaseCharacter.0BaseCharacter_C")
          (Variables|ServerSettings|SetCanTheGameStart? false)
          (CallFunction|CannotStart)
          (else
            (Variables|ServerSettings|SetCanTheGameStart? true)))))))

(event Custom|RespawnPlayer
  (params (Player%20Controller :type Player%20Controller%20Object%20Reference))
  (bind _returnvalue (Pawn|GetControlledPawn Player%20Controller))
  (bind _spawnpoints (Variables|ServerSettings|GetSpawnPoints))
  ;[1 1 1] Spawn Player as Base Character when joined the lobby
  (Utilities|IsValid _returnvalue
    (:Is%20Valid
      (Actor|DestroyActor _returnvalue))
    (:Is%20Not%20Valid
      _))
  (bind _returnvalue_2 (Game|SpawnActorfromClass "/Game/Blueprints/Characters/0BaseCharacter.0BaseCharacter_C" (Transformation|GetActorTransform (Utilities|Array|Get(acopy) _spawnpoints (Math|Random|RandomIntegerinRange 0 (- (Utilities|Array|Length _spawnpoints) 1)))) "Undefined" 0 0))
  (Pawn|Possess Player%20Controller _returnvalue_2)
  (CallFunction|EveryoneUpdate))

(event Custom|YouHaveBeenKicked
  (params (Player%20ID :type Integer))
  ;[1 1 1] Kick Selected Player
  (Default|Kicked (.AsLobby%20PC (Utilities|Casting|CastToLobbyPC (Utilities|Array|Get(acopy) (Variables|ServerSettings|GetAllPlayerControllers) Player%20ID)))))

(event Custom|LaunchGame
  (bind _returnvalue (Game|GetPlayerController 0))
  ;[1 1 1] Map Selection
  (switch int (Variables|ServerSettings|GetGM%20Map%20ID)
    (:0
      (Development|ExecuteConsoleCommand "servertravel /Game/Maps/Map01" _returnvalue))
    (:1
      (Development|ExecuteConsoleCommand "servertravel /Game/Maps/Map02" _returnvalue))))

(event Custom|AddToKickList
  ;[1 1 1] Adds Player to kick list whilst in kick menu
  (bind _aslobby_pc (Utilities|Casting|CastToLobbyPC (Game|GetPlayerController 0)))
  (Utilities|IsValid (Variables|/Game/Blueprints/Lobby/LobbyPC.LobbyPC_C|GetLobbyMenyWB _aslobby_pc)
    (:Is%20Valid
      (if (Widget|IsVisible (Variables|/Game/UserInterface/Lobby/LobbyMenu.LobbyMenu_C|GetGameSettings (Variables|/Game/Blueprints/Lobby/LobbyPC.LobbyPC_C|GetLobbyMenyWB _aslobby_pc)))
        (Default|FillPlayersWindow (Variables|/Game/UserInterface/Lobby/LobbyMenu.LobbyMenu_C|GetGameSettings (Variables|/Game/Blueprints/Lobby/LobbyPC.LobbyPC_C|GetLobbyMenyWB _aslobby_pc)))))))

(event Custom|CannotStart
  ;[1 1 1] Updates on connected player's lobby info
  (Utilities|Array|ForEachLoopwithBreak (Variables|ServerSettings|GetConnectedPlayers)) ; enters at Break
)

(event Custom|ServerUpdate%20GameSettings
  (params (Map%20Image :type Texture%202D%20Object%20Reference) (Map%20Name :type Text) (Map%20Time :type Text) (MapID :type Integer))
  ;[1 1 1] Server Changes Passed to Client Lobbies
  (Variables|ServerSettings|SetGM%20Map%20Image Map%20Image)
  (Variables|ServerSettings|SetGM%20Map%20Name Map%20Name)
  (Variables|ServerSettings|SetGM%20Map%20Time Map%20Time)
  (Variables|ServerSettings|SetGM%20Map%20ID MapID)
  (for _array_element (Variables|ServerSettings|GetAllPlayerControllers)
    (bind _aslobby_pc (Utilities|Casting|CastToLobbyPC _array_element))
    (Default|UpdateLobbySettings _aslobby_pc (Variables|ServerSettings|GetGM%20Map%20Image) (Variables|ServerSettings|GetGM%20Map%20Name) (Variables|ServerSettings|GetGM%20Map%20Time))))

(event EventPostLogin
  (params (NewPlayer :type Player%20Controller%20Object%20Reference))
  ;[1 1 1] Initial Setup - Lobby / Respawn
  (Networking|SwitchHasAuthority
    (:Authority
      (Utilities|Array|Add (Variables|ServerSettings|GetAllPlayerControllers) NewPlayer)
      (bind _outactors (Actor|GetAllActorsOfClass "/Script/Engine.PlayerStart"))
      (Variables|ServerSettings|SetSpawnPoints _outactors)
      (bind _asgame_info_instance (Utilities|Casting|CastToGameInfoInstance (Game|GetGameInstance)))
      (Variables|ServerSettings|SetServer%20Name (Variables|/Game/Blueprints/Levels/GameInfoInstance.GameInfoInstance_C|GetServerName _asgame_info_instance))
      (Variables|ServerSettings|SetMax%20Players (Variables|/Game/Blueprints/Levels/GameInfoInstance.GameInfoInstance_C|GetMaxPlayers _asgame_info_instance))
      (bind _aslobby_pc (Utilities|Casting|CastToLobbyPC NewPlayer))
      (Default|InitialSetup _aslobby_pc)
      (Default|SetupLobbyMenu _aslobby_pc (Variables|ServerSettings|GetServer%20Name))
      (Default|UpdateLobbySettings _aslobby_pc (Variables|ServerSettings|GetGM%20Map%20Image) (Variables|ServerSettings|GetGM%20Map%20Name) (Variables|ServerSettings|GetGM%20Map%20Time))
      (CallFunction|RespawnPlayer NewPlayer))))

(event EventOnLogout
  (params (ExitingController :type Controller%20Object%20Reference))
  (bind _allplayercontrollers (Variables|ServerSettings|GetAllPlayerControllers))
  ;[1 1 1] On Logout Removes player controller + info, makes their character available
  (bind (_array_element _array_index) (Utilities|Array|ForEachLoopwithBreak _allplayercontrollers :!label _label)
    (:LoopBody
      (if (== _array_element ExitingController)
        (goto _label Break)))
    (:Completed
      (bind _aslobby_pc (Utilities|Casting|CastToLobbyPC (Utilities|Array|Get(acopy) _allplayercontrollers _array_index)))
      (Utilities|Array|SetArrayElem (Variables|ServerSettings|GetAvailable%20Characters) (Variables|/Game/Blueprints/Lobby/LobbyPC.LobbyPC_C|GetSelected%20Character _aslobby_pc) false)
      (Utilities|Array|RemoveIndex (Variables|ServerSettings|GetAllPlayerControllers) _array_index)
      (Utilities|Array|RemoveIndex (Variables|ServerSettings|GetConnectedPlayers) _array_index)
      (CallFunction|EveryoneUpdate))))

(fn ConstructionScript)