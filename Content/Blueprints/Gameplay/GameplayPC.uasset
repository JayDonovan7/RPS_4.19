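; Gameplay player controller that handles character spawning and text chat for a multiplayer game.
; On BeginPlay the local controller loads saved player settings and passes them on, so GameplayGM respawns the chosen character and the chat widget is created.
; Chat messages are tagged with the player's name and relayed through the game mode's controller list to update each player's chat window.
; The T key toggles the mouse cursor.
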(event Custom|Pass%20Character%20info
  (params (Player%20Settings%20Info :type Player%20Info%20Structure))
  ;[1 1 1] Passes Character Info - Respawn Player - Set up chat window
  (Variables|Default|SetPlayer%20Settings Player%20Settings%20Info)
  (bind _asgameplay_gm (Utilities|Casting|CastToGameplayGM (Game|GetGameMode)))
  (Default|RespawnPlayer _asgameplay_gm self (.MyPlayerCharacter (Utilities|Struct|BreakPlayerInfo (Variables|Default|GetPlayer%20Settings))))
  (CallFunction|ChatWindow))

(event Custom|Get%20chat%20message
  (params (TextToSend :type Text))
  ;[1 1 1] Updaest chat on incoming message on the client
  (Variables|Default|SetSender%20Text TextToSend)
  (Variables|Default|SetSender%20Name (.MyPlayerName (Utilities|Struct|BreakPlayerInfo (Variables|Default|GetPlayer%20Settings))))
  (bind _asgameplay_gm (Utilities|Casting|CastToGameplayGM (Game|GetGameMode)))
  (for _array_element (Variables|/Game/Blueprints/Gameplay/GameplayGM.GameplayGM_C|GetAllPlayerControllers _asgameplay_gm)
    (bind _asgameplay_pc (Utilities|Casting|CastToGameplayPC _array_element))
    (CallFunction|UpdateChat _asgameplay_pc (Variables|Default|GetSender%20Name) (Variables|Default|GetSender%20Text))))

(event Custom|Update%20Chat
  (params (Sender%20Name :type Text) (Sender%20Text :type Text))
  ;[1 1 1] Update Client Chat Window
  (Default|UpdateChatWindow (Variables|/Game/UserInterface/Levels/GameplayChat.GameplayChat_C|GetGameplayChat (Variables|Default|GetGameplay%20chat%20WB)) Sender%20Name Sender%20Text))

(event Custom|Chat%20Window
  ;[1 1 1] Add chat to the viewport
  (bind _returnvalue (UserInterface|CreateWidget "/Game/UserInterface/Levels/GameplayChat.GameplayChat_C"))
  (bind _output_get (Variables|Default|SetGameplay%20chat%20WB _returnvalue))
  (UserInterface|Viewport|AddtoViewport _output_get 0))

(event EventBeginPlay
  ;[1 1 1] Load Player Info and pass it to server player controler
  (if (Pawn|IsLocalController)
    (Viewport|RemoveAllWidgets)
    (CallFunction|LoadGame)
    (CallFunction|PassCharacterInfo (Variables|Default|GetPlayer%20Settings))))

(event Input|KeyboardEvents|T
  (params (Key :type Key%20Structure))
  ;[1 0 0] Type
  (:Pressed
    (Utilities|FlowControl|FlipFlop
      (:A
        (Variables|Default|SetbShowMouseCursor true))
      (:B
        (Variables|Default|SetbShowMouseCursor false)))))

(event Input|KeyboardEvents|Tab
  (params (Key :type Key%20Structure))
  ;[1 0 0] Type
)

(fn ConstructionScript)

(fn LoadGame
  (bind _returnvalue (SaveGame|LoadGamefromSlot (Variables|Default|GetPlayerSettingsSave)))
  (bind _asplayer_save_info (Utilities|Casting|CastToPlayerSaveInfo _returnvalue))
  (Variables|Default|SetPlayer%20Settings (Variables|/Game/Blueprints/Levels/PlayerSaveInfo.PlayerSaveInfo_C|GetS_PlayerInfo _asplayer_save_info)))