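; Game mode for the RPS multiplayer test that creates local players and swaps their pawns between playing and despawned states.
; BeginPlay caches all PlayerStarts and calls CreatePlayer until its player counter exceeds three.
; SpawnPlayer and DespawnPlayer replace an existing pawn with BaseCharacter or Pawn01, possess it, and show or remove the controller's HUD.
; Both spawn at GetRandomSpawn, whose random PlayerStart lookup appears unconnected.
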(event Custom|SpawnPlayer
  (params (Player%20Controller :type Player%20Controller%20Object%20Reference))
  (bind _returnvalue (Pawn|GetControlledPawn Player%20Controller))
  (Utilities|IsValid _returnvalue
    (:Is%20Valid
      (Actor|DestroyActor _returnvalue)
      (bind _returnvalue_2 (Game|SpawnActorfromClass "/Game/Character/BaseCharacter.BaseCharacter_C" (Utilities|GetRandomSpawn) "Undefined" 0 0))
      (Pawn|Possess Player%20Controller _returnvalue_2)
      (UserInterface|Viewport|AddtoPlayerScreen (Variables|/Game/MultiplayerTest/Blueprints/RPS-Controller.RPS-Controller_C|GetHUD (.AsRPS-Controller (Utilities|Casting|CastToRPS-Controller Player%20Controller)))))))

(event Custom|Despawn%20Player
  (params (Player%20Controller :type Player%20Controller%20Object%20Reference))
  (bind _returnvalue (Pawn|GetControlledPawn Player%20Controller))
  (Utilities|IsValid _returnvalue
    (:Is%20Valid
      (Actor|DestroyActor _returnvalue)
      (bind _returnvalue_2 (Game|SpawnActorfromClass "/Game/Character/Pawn01.Pawn01_C" (Utilities|GetRandomSpawn) "Undefined" 0 0))
      (Pawn|Possess Player%20Controller _returnvalue_2)
      (Widget|RemovefromParent (Variables|/Game/MultiplayerTest/Blueprints/RPS-Controller.RPS-Controller_C|GetHUD (.AsRPS-Controller (Utilities|Casting|CastToRPS-Controller Player%20Controller)))))))

(event EventBeginPlay
  (bind _outactors (Actor|GetAllActorsOfClass "/Script/Engine.PlayerStart"))
  (Variables|Default|SetSpawnPoints _outactors)
  (while (<= (Variables|Default|GetNumberOfPlayers) 3)
    (Variables|Default|SetNumberOfPlayers (+ (Variables|Default|GetNumberOfPlayers) 1))
    (Class|GameplayStatics|CreatePlayer -1)))

(fn ConstructionScript)