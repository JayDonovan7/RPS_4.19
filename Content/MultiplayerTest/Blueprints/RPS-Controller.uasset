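; RPS player controller that creates a HUD widget and lets its player request spawning or despawning through input.
; On BeginPlay it creates the widget with itself as owner and stores it, without adding it to the viewport here.
; Key 1 or gamepad Start calls SpawnPlayer on RPS-GameModeMain, while key 2 or Select calls DespawnPlayer, each passing this controller.
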(event EventBeginPlay
  (bind _returnvalue (UserInterface|CreateWidget "/Game/UserInterface/HUD.HUD_C" self))
  (Variables|Default|SetHUD _returnvalue))

(event Input|GamepadEvents|GamepadSpecialLeft
  (params (Key :type Key%20Structure :default "AnyKey"))
  ;[1 1 1] Select
  (:Pressed
    (bind _asrps_game_mode_main (Utilities|Casting|CastToRPS-GameModeMain (Game|GetGameMode)))
    (Default|DespawnPlayer _asrps_game_mode_main self)))

(event Input|GamepadEvents|GamepadSpecialRight
  (params (Key :type Key%20Structure :default "AnyKey"))
  ;[1 1 1] start
  (:Pressed
    (bind _asrps_game_mode_main (Utilities|Casting|CastToRPS-GameModeMain (Game|GetGameMode)))
    (Default|SpawnPlayer _asrps_game_mode_main self)))

(event Input|KeyboardEvents|1
  (params (Key :type Key%20Structure :default "AnyKey"))
  (:Pressed
    (bind _asrps_game_mode_main (Utilities|Casting|CastToRPS-GameModeMain (Game|GetGameMode)))
    (Default|SpawnPlayer _asrps_game_mode_main self)))

(event Input|KeyboardEvents|2
  (params (Key :type Key%20Structure :default "AnyKey"))
  (:Pressed
    (bind _asrps_game_mode_main (Utilities|Casting|CastToRPS-GameModeMain (Game|GetGameMode)))
    (Default|DespawnPlayer _asrps_game_mode_main self)))

(fn ConstructionScript)